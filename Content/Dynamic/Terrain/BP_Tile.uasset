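; Infinite-terrain tile that acts as a locked room, populated with random props and AI enemies whose count grows with conquered tiles.
; Player entry into LockingVolume picks an assassination or artefact-rescue mission, unless the tile has a persistent barrier.
; OnTileConquered turns the barrier green and passable; leaving the volume relocks it and reports the conquest to the game mode.
; GCVolume overlap makes the game mode spawn another tile and destroys this one.
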(event OnComponentBeginOverlap(Lockingvolume)
  (params (OverlappedComponent :type Primitive%20Component%20Object%20Reference) (OtherActor :type Actor%20Object%20Reference) (OtherComp :type Primitive%20Component%20Object%20Reference) (OtherBodyIndex :type Integer) (bFromSweep :type Boolean) (SweepResult :type Hit%20Result%20Structure%20%28by%20ref%29))
  (Utilities|IsPlayerActor OtherActor
    (:true
      (if (not (Variables|Default|GetPersistentBarrier))
        (CallFunction|GenerateConquerCondition)))))

(event OnComponentEndOverlap(Lockingvolume)
  (params (OverlappedComponent :type Primitive%20Component%20Object%20Reference) (OtherActor :type Actor%20Object%20Reference) (OtherComp :type Primitive%20Component%20Object%20Reference) (OtherBodyIndex :type Integer))
  (Utilities|IsPlayerActor OtherActor
    (:true
      (CallFunction|Lock (Variables|Default|GetBarrier))
      (CallFunction|ConquerTile))))

(event OnComponentBeginOverlap(GCVolume)
  (params (OverlappedComponent :type Primitive%20Component%20Object%20Reference) (OtherActor :type Actor%20Object%20Reference) (OtherComp :type Primitive%20Component%20Object%20Reference) (OtherBodyIndex :type Integer) (bFromSweep :type Boolean) (SweepResult :type Hit%20Result%20Structure%20%28by%20ref%29))
  (Utilities|IsPlayerActor OtherActor
    (:true
      (bind _asinfinite_terrain_game_mode_bp (Utilities|Casting|CastToInfiniteTerrainGameMode_BP (Game|GetGameMode)))
      (Default|SpawnTile _asinfinite_terrain_game_mode_bp)
      (Actor|DestroyActor))))

(event EventBeginPlay
  (bind _returnvalue (Class|Tile|GetConquerCondition))
  (if (Utilities|Enum|Equal(Enum) _returnvalue "None")
    (CallFunction|Unlock)
    (else
      (CallFunction|Lock (Variables|Default|GetBarrier))))
  (Utilities|FlowControl|Sequence
    (:then_0
      (if (Variables|Default|GetPersistentBarrier)
        (CallFunction|SpawnPersistentBarrier)))
    (:then_1
      (if (Variables|Default|GetSpawnProps)
        (CallFunction|SpawnRandomObjects)))
    (:then_2
      (if (Variables|Default|GetSpawn%20AI)
        (bind (_returnvalue_2 _returnvalue2) (CallFunction|GetNumberOfEnemies))
        (Class|Tile|PlaceAiPawns "/Game/Dynamic/Character/Behaviour/BP_Character.BP_Character_C" _returnvalue_2 _returnvalue2 1.5e+02)))))

(event EventOnTileConquered
  (bind _returnvalue (Game|GetPlayerController 0))
  (CallFunction|Unlock)
  (Utilities|IsValid _returnvalue
    (:Is%20Valid
      (bind _asbp_hud (Utilities|Casting|CastToBP_HUD (HUD|GetHUD _returnvalue)))
      (Default|ShowMissionText _asbp_hud "ROOM UNLOCKED"))))

(fn ConstructionScript)

(fn GetAttachLocation
  (return (Transformation|GetWorldTransform (Variables|Default|GetArrow))))

(fn Unlock
  (Collision|SetCollisionObjectType (Variables|Default|GetBarrier) "ECC_GameTraceChannel3")
  (Rendering|Material|SetMaterial (Variables|Default|GetBarrier) 0 "/Game/Dynamic/Terrain/MI_Barrier_Green.MI_Barrier_Green"))

(fn Lock
  (params (Barrier :type Primitive%20Component%20Object%20Reference))
  (Utilities|IsValid Barrier
    (:Is%20Valid
      (Collision|SetCollisionObjectType Barrier "ECC_WorldStatic")
      (Rendering|Material|SetMaterial Barrier 0 "/Game/Dynamic/Terrain/MI_Barrier_Red.MI_Barrier_Red"))))

(fn ConquerTile
  (bind _returnvalue (Class|Tile|IsTileConquered))
  (if (not _returnvalue)
    (Class|Tile|SetConqueredTile)
    (bind _asinfinite_terrain_game_mode_bp (Utilities|Casting|CastToInfiniteTerrainGameMode_BP (Game|GetGameMode)))
    (Class|InfiniteTerrainGameMode|TileConquered _asinfinite_terrain_game_mode_bp)))

(fn SpawnPersistentBarrier
  (bind _returnvalue (Game|SpawnActorfromClass "/Game/Dynamic/Terrain/Props/BP_Barrier.BP_Barrier_C" (Transformation|GetWorldTransform (Variables|Default|GetBarrierSpawnPoint)) "Undefined" 0 0))
  (CallFunction|Lock (Variables|/Game/Dynamic/Terrain/Props/BP_Barrier.BP_Barrier_C|GetStaticMesh _returnvalue)))

(fn PlaceActors
  (params (ToSpawn :type Actor%20Class%20Reference) (MinSpawn :type Integer) (MaxSpawn :type Integer))
  (Class|Tile|PlaceActors ToSpawn MinSpawn MaxSpawn 4e+02 1.0 1.0 false))

(fn PlaceAIPawns
  (params (ToSpawn :type Pawn%20Class%20Reference) (MinSpawn :type Integer) (MaxSpawn :type Integer) (Radius :type Float%20%28single-precision%29))
  (Class|Tile|PlaceAiPawns ToSpawn MinSpawn MaxSpawn Radius))

(fn SpawnRandomObjects
  (Class|Tile|PlaceActors "/Game/Dynamic/Terrain/Props/BP_Container.BP_Container_C" 2 5 5e+02 1.0 1.0 false)
  (Class|Tile|PlaceActors "/Game/Dynamic/Terrain/Props/BP_Canister.BP_Canister_C" 0 2 75.0 1.0 1.0 false)
  (Class|Tile|PlaceActors "/Game/Dynamic/Terrain/Props/BP_Rock02.BP_Rock02_C" 1 3 2.5e+02 1.0 3.0 false)
  (Class|Tile|PlaceActors "/Game/Dynamic/Terrain/Props/BP_Rock03.BP_Rock03_C" 2 5 3.5e+02 1.0 3.0 false))

(fn GenerateConquerCondition
  (bind _maxquestitems (Variables|Default|GetMaxQuestItems))
  (bind _output_get (Variables|Default|SetMissionType (Utilities|Enum|ByteToEnumEConquerCondition (Math|Conversions|ToByte(Integer) (Math|Random|RandomInteger 2)))))
  (Class|Tile|SetConquerCondition _output_get)
  (switch Utilities|FlowControl|Switch|SwitchonEConquerCondition _output_get
    (:Assassination
      (CallFunction|ShowMissionText "KILL ALL THE GUARDS"))
    (:Rescue
      (CallFunction|ShowMissionText (Utilities|String|Append (Utilities|String|MakeLiteralString "RESCUE ") (Utilities|String|ToString(Integer) (Variables|Default|GetMaxQuestItems)) (Utilities|String|MakeLiteralString " ARTEFACTS")))
      (Class|Tile|PlaceActors "/Game/Dynamic/Terrain/Props/BP_ItemAltar.BP_ItemAltar_C" _maxquestitems _maxquestitems 1.5e+02 1.0 1.0 true))))

(fn ShowMissionText
  (params (Text :type String))
  (bind _asbp_hud (Utilities|Casting|CastToBP_HUD (HUD|GetHUD (Game|GetPlayerController 0))))
  (Default|ShowMissionText _asbp_hud Text))

(fn GetNumberOfEnemies
  (bind _asinfinite_terrain_game_mode_bp (Utilities|Casting|CastToInfiniteTerrainGameMode_BP (Game|GetGameMode))
    (:then
      _)
    (:CastFailed
      _))
  (return (+ (Variables|Default|GetMinEnemySpawn) (Class|InfiniteTerrainGameMode|GetNumberOfConqueredTiles _asinfinite_terrain_game_mode_bp)) (+ (Class|InfiniteTerrainGameMode|GetNumberOfConqueredTiles _asinfinite_terrain_game_mode_bp) (Variables|Default|GetMaxEnemySpawn))))