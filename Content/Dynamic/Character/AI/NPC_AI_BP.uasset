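; AI controller Blueprint for guard NPCs that drives the GuardBehaviour behavior tree with the PatrolData blackboard.
; On BeginPlay it sets up the blackboard, starts the tree and caches the blackboard component.
; AI Perception updates write a sensed actor to the enemy key, or clear the key when sensing fails.
; Actors tagged "Enemy" are ignored, so they neither set nor clear that key.
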(event OnTargetPerceptionUpdated(AIPerception)
  (params (Actor :type Actor%20Object%20Reference) (Stimulus :type AI%20Stimulus%20Structure))
  (CallFunction|UpdateBlackBoardEnemyKey (.bsuccessfullysensed Stimulus) Actor Actor))

(event EventBeginPlay
  (bind _blackboardcomponent (Class|AIController|UseBlackboard "/Game/Dynamic/Character/AI/PatrolData.PatrolData"))
  (AI|RunBehaviorTree "/Game/Dynamic/Character/AI/GuardBehaviour.GuardBehaviour")
  (Variables|Default|SetBlackboardComp _blackboardcomponent))

(fn ConstructionScript)

(fn UpdateBlackBoardEnemyKey
  (params (Condition :type Boolean) (Target :type Actor%20Object%20Reference) (self2 :type Actor%20Object%20Reference))
  (if (not (Actor|ActorHasTag self2 "Enemy"))
    (if Condition
      (bind _output_get (Variables|Default|SetTarget Target))
      (AI|Components|Blackboard|SetValueasObject (Variables|Default|GetBlackboardComp) (Variables|Default|GetEnemyKey) _output_get)
      (else
        (AI|Components|Blackboard|ClearValue (Variables|Default|GetBlackboardComp) (Variables|Default|GetEnemyKey))))))