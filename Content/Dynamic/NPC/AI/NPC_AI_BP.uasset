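; AI Controller for guard NPCs that feeds perceived targets into their behavior tree.
; On BeginPlay it initializes the PatrolData blackboard and runs the GuardBehaviour tree.
; AI Perception updates ignore actors tagged "Enemy", storing any other sensed actor as Target and in the blackboard's enemy key.
; A failed sense of any such actor clears that key, without checking whether it is the current target.
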(event OnTargetPerceptionUpdated(AIPerception)
  (params (Actor :type Actor%20Object%20Reference) (Stimulus :type AI%20Stimulus%20Structure))
  (if (not (Actor|ActorHasTag Actor "Enemy"))
    (if (.bsuccessfullysensed Stimulus)
      (bind _output_get (Variables|Default|SetTarget Actor))
      (AI|Components|Blackboard|SetValueasObject (Variables|Default|GetBlackboardComp) (Variables|Default|GetEnemyKey) _output_get)
      (else
        (AI|Components|Blackboard|ClearValue (Variables|Default|GetBlackboardComp) (Variables|Default|GetEnemyKey))))))

(event EventBeginPlay
  (bind _blackboardcomponent (Class|AIController|UseBlackboard "/Game/Dynamic/NPC/AI/PatrolData.PatrolData"))
  (AI|RunBehaviorTree "/Game/Dynamic/NPC/AI/GuardBehaviour.GuardBehaviour")
  (Variables|Default|SetBlackboardComp _blackboardcomponent))

(fn ConstructionScript)